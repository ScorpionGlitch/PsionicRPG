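; AI controller for non-player characters that patrol, spot the player and investigate stimuli.
; On possession it runs BT_NonPlayerCharacter and seeds the blackboard with the pawn's patrol path loop and wait settings plus a starting direction.
; Perception updates route each stimulus by array index to sight, hearing or damage handlers.
; Sight sets CanSeePlayer; hearing and damage set IsInvestigating and, when sensed, the Destination location.
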(event `self.ReceivePossess`
  (params (PossessedPawn :type "Pawn Object Reference"))
  (`self.RunBehaviorTree` "/Game/AI/BT_NonPlayerCharacter.BT_NonPlayerCharacter")
  (bind _asbp_non_player_character (cast `/Game/Characters/NonPlayerCharacters/BP_NonPlayerCharacter` (`self.K2_GetPawn`)))
  (bind _output_get (set `self.NonPlayerCharacter` _asbp_non_player_character))
  (bind _patrolpath (`/Game/Characters/NonPlayerCharacters/BP_NonPlayerCharacter.PatrolPath` _output_get))
  (`BlackboardComponent.SetValueAsBool` (`AIBlueprintHelperLibrary.GetBlackboard` null) "IsLooping" (`/Game/AI/PatrolPath.IsLooping` _patrolpath))
  (`BlackboardComponent.SetValueAsFloat` (`AIBlueprintHelperLibrary.GetBlackboard` null) "WaitTime" (`/Game/AI/PatrolPath.WaitTime` _patrolpath))
  (`BlackboardComponent.SetValueAsInt` (`AIBlueprintHelperLibrary.GetBlackboard` null) "Direction" 1))

(event `self.AIPerception.OnPerceptionUpdated`
  (params (UpdatedActors :type "Array of Actor Object Reference (by ref)"))
  (for _array_element UpdatedActors
    (bind _info (`AIPerceptionComponent.GetActorsPerception` (`self.AIPerception`) _array_element))
    (for (_array_element_2 _array_index) (`.LastSensedStimuli` (break `ActorPerceptionBlueprintInfo` _info))
      (switch `int` _array_index
        (:`0`
          (`self.ProcessVisualSense` _array_element_2))
        (:`1`
          (`self.ProcessAudioSense` _array_element_2))
        (:`2`
          (`self.ProcessDamageSense` _array_element_2))))))

(fn `ProcessAudioSense`
  (params (AIStimulus :type "AIStimulus Structure"))
  (bind (_aistimulus_age _aistimulus_expirationage _aistimulus_strength _aistimulus_stimuluslocation _aistimulus_receiverlocation _aistimulus_tag _aistimulus_bsuccessfullysensed) (break `AIStimulus` (`local.AIStimulus`)))
  (`BlackboardComponent.SetValueAsBool` (`AIBlueprintHelperLibrary.GetBlackboard` null) "IsInvestigating" _aistimulus_bsuccessfullysensed)
  (if _aistimulus_bsuccessfullysensed
    (`BlackboardComponent.SetValueAsVector` (`AIBlueprintHelperLibrary.GetBlackboard` null) "Destination" _aistimulus_stimuluslocation)))

(fn `ProcessDamageSense`
  (params (AIStimulus :type "AIStimulus Structure"))
  (bind (_aistimulus_age _aistimulus_expirationage _aistimulus_strength _aistimulus_stimuluslocation _aistimulus_receiverlocation _aistimulus_tag _aistimulus_bsuccessfullysensed) (break `AIStimulus` (`local.AIStimulus`)))
  (`BlackboardComponent.SetValueAsBool` (`AIBlueprintHelperLibrary.GetBlackboard` null) "IsInvestigating" _aistimulus_bsuccessfullysensed)
  (if _aistimulus_bsuccessfullysensed
    (`BlackboardComponent.SetValueAsVector` (`AIBlueprintHelperLibrary.GetBlackboard` null) "Destination" _aistimulus_stimuluslocation)))

(fn `ProcessVisualSense`
  (params (AIStimulus :type "AIStimulus Structure"))
  (bind (_aistimulus_age _aistimulus_expirationage _aistimulus_strength _aistimulus_stimuluslocation _aistimulus_receiverlocation _aistimulus_tag _aistimulus_bsuccessfullysensed) (break `AIStimulus` (`local.AIStimulus`)))
  (`BlackboardComponent.SetValueAsBool` (`AIBlueprintHelperLibrary.GetBlackboard` null) "CanSeePlayer" _aistimulus_bsuccessfullysensed))

(fn `UserConstructionScript`)